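; Baker NPC actor that sells bread for the player's coins, "pooping" out each loaf with a fart sound.
; A trigger shows the purchase prompt, and DoPurchase spends a coin and sets IsPooping, with a short delay on the first buy of each visit.
; DoPoop spawns a randomly scaled BP_Bread, launches it relative to the skeletal mesh and clears the flag.
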(event `self.ReceiveBeginPlay`
  ;[1 0 0.8696] Init
  (`self.EnableInput` (`GameplayStatics.GetPlayerController` 0)))

(event `self.Trigger.OnComponentBeginOverlap`
  (params (OverlappedComponent :type "PrimitiveComponent Object Reference") (OtherActor :type "Actor Object Reference") (OtherComp :type "PrimitiveComponent Object Reference") (OtherBodyIndex :type Integer) (bFromSweep :type Boolean) (SweepResult :type "HitResult Structure (by ref)"))
  (cast `/Game/Baker/Blueprints/BP_Player` (`GameplayStatics.GetPlayerCharacter` 0))
  (`SceneComponent.SetVisibility` (`self.PressToBuy`) true false))

(event `self.Trigger.OnComponentEndOverlap`
  (params (OverlappedComponent :type "PrimitiveComponent Object Reference") (OtherActor :type "Actor Object Reference") (OtherComp :type "PrimitiveComponent Object Reference") (OtherBodyIndex :type Integer))
  (cast `/Game/Baker/Blueprints/BP_Player` (`GameplayStatics.GetPlayerCharacter` 0))
  (`SceneComponent.SetVisibility` (`self.PressToBuy`) false false)
  (set `self.inPurchaseMode` false))

(event `DoPurchase`
  (bind _returnvalue (`GameplayStatics.GetPlayerCharacter` 0))
  ;[1 0.3646 0.3646] Activate Purchase
  (if (`PrimitiveComponent.IsOverlappingActor` (`self.Trigger`) _returnvalue)
    (bind _asbp_player (cast `/Game/Baker/Blueprints/BP_Player` _returnvalue))
    (bind _coincount (`/Game/Baker/Blueprints/BP_Player.CoinCount` _asbp_player))
    (if (> _coincount 0)
      (if (`self.inPurchaseMode`)
        (if (not (`self.isPooping`))
          (set `self.isPooping` true :!label _label)
          (set `/Game/Baker/Blueprints/BP_Player.CoinCount` (+ _coincount -1) _asbp_player))
        (else
          (set `self.inPurchaseMode` true)
          (`KismetSystemLibrary.Delay` 0.5)
          (goto _label))))))

(event `DoPoop`
  (bind (_returnvalue_location _returnvalue_rotation) (`KismetMathLibrary.BreakTransform` (`SceneComponent.GetRelativeTransform` (`self.SkeletalMesh`))))
  (bind (_returnvalue_location_2 _returnvalue_rotation_2) (`KismetMathLibrary.BreakTransform` (`SceneComponent.GetRelativeTransform` (`self.SkeletalMesh`))))
  ;[1 0.3125 0.3125] POOP
  (bind _returnvalue (`|SpawnActorFromClass` "/Game/Baker/Blueprints/BP_Bread.BP_Bread_C" (`KismetMathLibrary.MakeTransform` (`KismetMathLibrary.TransformLocation` (`KismetMathLibrary.MakeTransform` _returnvalue_location_2 _returnvalue_rotation_2) (0.0 -20.0 75.0)) (`KismetMathLibrary.ComposeRotators` _returnvalue_rotation_2 (struct :`Yaw` 90.0)) (* (1.0 1.0 1.0) (`KismetMathLibrary.RandomFloatInRange` 0.5 2.0))) "AlwaysSpawn" "OverrideRootScale" null null))
  (`PrimitiveComponent.SetPhysicsLinearVelocity` (`/Game/Baker/Blueprints/BP_Bread.StaticMesh` _returnvalue) (`KismetMathLibrary.TransformLocation` (`KismetMathLibrary.MakeTransform` _returnvalue_location _returnvalue_rotation) (0.0 -250.0 50.0)) false "None")
  (`GameplayStatics.PlaySound2D` "/Game/Baker/Sounds/SND_Fart.SND_Fart")
  (set `self.isPooping` false))

(fn `UserConstructionScript`
  (`SceneComponent.SetVisibility` (`self.PressToBuy`) false false))